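; Weather manager that switches between six states from clear to heavy storm and fog, instantly or through Timeline blends with change events.
; Weather intensity and per-state targets drive weather and ocean parameter collections, height fog, sun, skylight and rain.
; Niagara rain follows the player on a timer and receives OceanManager wave data each tick while active.
; Storm intensity schedules random lightning around the player, with thunder delayed by distance at sound speed.
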(event Custom|TransitionToWeather
  (params (NewWeather :type E_WeatherType%20Enum :default "NewEnumerator0") (Duration :type Float%20%28double-precision%29))
  (if (<= Duration 0.01)
    (CallFunction|SetWeatherInstant NewWeather)
    (else
      (Variables|Transition|SetStartingWeatherIntensity (Variables|WeatherTypes|GetWeatherIntensity))
      (Variables|WeatherTypes|SetTargetWeather NewWeather)
      (CallFunction|SetTransitionValues)
      (Variables|Transition|SetTransitionDuration Duration)
      (Variables|Transition|SetTransitionProgress 0.0)
      (Variables|Transition|SetIsTransitioning true)
      (bind _intensity (CallFunction|GetIntensityforWeather (Variables|WeatherTypes|GetTargetWeather)))
      (Variables|Transition|SetTargetWeatherIntensity _intensity)
      (Default|CallOnWeatherTransitionStarted (Variables|WeatherTypes|GetCurrentWeather) (Variables|WeatherTypes|GetTargetWeather) (Variables|Transition|GetTransitionDuration))
      (Components|Timeline|SetPlayRate (Variables|Default|GetTI_WeatherTransition) (/ 1.0 (Variables|Transition|GetTransitionDuration)))
      (bind _transitionalpha (Timeline|TI_WeatherTransition PlayFromStart)
        (:Update
          (Variables|Transition|SetTransitionProgress _transitionalpha)
          (Variables|WeatherTypes|SetWeatherIntensity (Math|Float|Lerp (Variables|Transition|GetStartingWeatherIntensity) (Variables|Transition|GetTargetWeatherIntensity) (Variables|Transition|GetTransitionProgress)))
          (Variables|Fog|SetCurrentFogDensity (Math|Float|Lerp (Variables|Fog|GetStartFogDensity) (Variables|Fog|GetTargetFogDensity) (Variables|Transition|GetTransitionProgress)))
          (Variables|Fog|SetCurrentFogHeightFalloff (Math|Float|Lerp (Variables|Fog|GetStartFogHeightFalloff) (Variables|Fog|GetTargetFogHeightFalloff) (Variables|Transition|GetTransitionProgress)))
          (Variables|Light|SetCurrentSunIntensity (Math|Float|Lerp (Variables|Light|GetStartSunIntensity) (Variables|Light|GetTargetSunIntensity) (Variables|Transition|GetTransitionProgress)))
          (Variables|Light|SetCurrentSkyLightIntensity (Math|Float|Lerp (Variables|Light|GetStartSkyLightIntensity) (Variables|Light|GetTargetSkyLightIntensity) (Variables|Transition|GetTransitionProgress)))
          (Variables|Clouds|SetCurrentCloudCoverage (Math|Float|Lerp (Variables|Clouds|GetStartCloudCoverage) (Variables|Clouds|GetTargetCloudCoverage) (Variables|Transition|GetTransitionProgress)))
          (Variables|Rain|SetCurrentRainIntensity (Math|Float|Lerp (Variables|Rain|GetStartRainIntensity) (Variables|Rain|GetTargetRainIntensity) (Variables|Transition|GetTransitionProgress)))
          (Variables|Clouds|SetCurrentStormCloudAmount (Math|Float|Lerp (Variables|Clouds|GetStartStormCloudAmount) (Variables|Clouds|GetTargetStormCloudAmount) (Variables|Transition|GetTransitionProgress)))
          (CallFunction|ApplyWeatherValues)
          (Default|CallOnWeatherIntensityChanged (Variables|WeatherTypes|GetWeatherIntensity)))
        (:Finished
          (Variables|WeatherTypes|SetWeatherIntensity (Variables|Transition|GetTargetWeatherIntensity))
          (Variables|WeatherTypes|SetCurrentWeather (Variables|WeatherTypes|GetTargetWeather))
          (Variables|Transition|SetTransitionProgress 1.0)
          (Variables|Transition|SetIsTransitioning false)
          (CallFunction|ApplyWeatherValues)
          (Default|CallOnWeatherChanged (Variables|WeatherTypes|GetCurrentWeather)))))))

(event Custom|RainFollowPlayer
  (bind _rainfollowtarget (Variables|Actors|GetRainFollowTarget))
  (bind _ns_rain (Variables|Default|GetNS_Rain))
  (bind _returnvalue (Transformation|GetActorLocation _rainfollowtarget))
  (Transformation|SetWorldLocation _ns_rain (Math|Vector|MakeVector (.x _returnvalue) (.y _returnvalue) (.z (Transformation|GetWorldLocation _ns_rain))) false false))

(event Custom|ThunderSFX
  (params (StrikeLocation :type Vector))
  (Utilities|FlowControl|Delay (/ (Math|Vector|Distance(Vector) StrikeLocation (Transformation|GetActorLocation (Game|Player|GetPlayerPawn 0))) 3.43e+04))
  (Audio|SpawnSoundatLocation "/Game/Sounds/Thunder/SC_Thunder.SC_Thunder" StrikeLocation "0, 0, 0" (Math|Random|RandomFloatinRange 0.85 1.15) (Math|Random|RandomFloatinRange 0.95 1.05) 0.0 "/Game/Sounds/Thunder/SA_Thunder.SA_Thunder" 0))

(event EventTick
  (params (DeltaSeconds :type Float%20%28single-precision%29))
  (if (Components|Activation|IsActive (Variables|Default|GetNS_Rain))
    (CallFunction|UpdateRainOceanParameters)
    (Niagara|SetNiagaraVariable(Float) (Variables|Default|GetNS_Rain) "User.GlobalWaveStrength" (Variables|/Game/Blueprints/Managers/BP_OceanManager.BP_OceanManager_C|GetGlobalWaveStrength (Variables|Actors|GetOceanManager)))
    (Niagara|SetNiagaraVariable(Float) (Variables|Default|GetNS_Rain) "User.OceanTime" (Variables|/Game/Blueprints/Managers/BP_OceanManager.BP_OceanManager_C|GetOceanTime (Variables|Actors|GetOceanManager)))
    (bind _returnvalue (Rendering|Material|GetScalarParameterValue "/Game/MaterialParameterCollections/MPC_Weather.MPC_Weather" "LightningIntensity" :!class /Script/Engine.KismetMaterialLibrary))
    (bind _output_get (Variables|Lightning|SetLightningIntensity _returnvalue))
    (if (> _output_get 0.01)
      (if (>= (Utilities|Time|GetGameTimeinSeconds) (Variables|Lightning|GetNextLightningTime))
        (bind _strikelocation (CallFunction|TriggerLightningStrike))
        (bind _output_get_2 (Variables|Lightning|SetLightningIntensity (Math|Float|Clamp(Float) (Variables|Lightning|GetLightningIntensity))))
        (Variables|Lightning|SetNextLightningTime (+ (* (Math|Float|Lerp 12.0 4.0 _output_get_2) (Math|Random|RandomFloatinRange 0.8 1.4)) (Utilities|Time|GetGameTimeinSeconds)))
        (CallFunction|ThunderSFX _strikelocation)))))

(event EventBeginPlay
  (CallFunction|SetWeatherInstant (Variables|WeatherTypes|GetStartingWeather))
  (Variables|Actors|SetRainFollowTarget (Game|GetPlayerCharacter 0))
  (Utilities|Time|SetTimerbyEvent (delegate Custom|RainFollowPlayer) 1.0 true)
  (bind _returnvalue (Actor|GetActorOfClass "/Game/Blueprints/Managers/BP_OceanManager.BP_OceanManager_C"))
  (bind _output_get (Variables|Actors|SetOceanManager _returnvalue))
  (Actor|Tick|AddTickPrerequisiteActor _output_get)
  (Actor|Tick|AddTickPrerequisiteActor (Variables|Default|GetNS_Rain) self)
  (Variables|Lightning|SetNextLightningTime 0.0))

(fn ConstructionScript)

(fn GetIntensityforWeather
  (params (Weather :type E_WeatherType%20Enum :default "NewEnumerator0"))
  (switch Utilities|FlowControl|Switch|SwitchonE_WeatherType Weather
    (:NewEnumerator0
      (return 0.0))
    (:NewEnumerator1
      (return 0.25))
    (:NewEnumerator2
      (return 0.5))
    (:NewEnumerator3
      (return 0.8))
    (:NewEnumerator4
      (return 1.0))
    (:NewEnumerator5
      (return 0.35))))

(fn ApplyWeatherValues
  (bind _heightfog (Variables|Actors|GetHeightFog))
  (bind _ns_rain (Variables|Default|GetNS_Rain))
  (bind _weatherintensity (Variables|WeatherTypes|GetWeatherIntensity))
  (bind _returnvalue (- _weatherintensity 0.35))
  (bind _component (Variables|/Script/Engine.ExponentialHeightFog|GetComponent _heightfog))
  (bind _returnvalue_2 (/ _returnvalue 0.65))
  (bind _returnvalue_3 (Math|Float|Clamp(Float) _returnvalue_2))
  (Rendering|Material|SetScalarParameterValue "/Game/MaterialParameterCollections/MPC_Weather.MPC_Weather" "WeatherIntensity" (Variables|WeatherTypes|GetWeatherIntensity) :!class /Script/Engine.KismetMaterialLibrary)
  (Rendering|Material|SetScalarParameterValue "/Game/MaterialParameterCollections/MPC_Weather.MPC_Weather" "WindStrength" (Math|Float|Lerp 0.05 1.0 (Variables|WeatherTypes|GetWeatherIntensity)) :!class /Script/Engine.KismetMaterialLibrary)
  (Rendering|Material|SetScalarParameterValue "/Game/MaterialParameterCollections/MPC_Weather.MPC_Weather" "CloudCoverage" (Math|Float|Lerp 0.05 1.0 (Variables|WeatherTypes|GetWeatherIntensity)) :!class /Script/Engine.KismetMaterialLibrary)
  (Rendering|Material|SetScalarParameterValue "/Game/MaterialParameterCollections/MPC_Weather.MPC_Weather" "RainIntensity" _returnvalue_3 :!class /Script/Engine.KismetMaterialLibrary)
  (if (> _returnvalue_3 0.0)
    (Components|Activation|Activate _ns_rain true)
    (else
      (Components|Activation|Deactivate _ns_rain)))
  (Niagara|SetNiagaraVariable(Float) _ns_rain "RainSpawnRate" (Math|Float|Lerp (Variables|Rain|GetMinRainSpawnRate) (Variables|Rain|GetMaxRainSpawnRate) _returnvalue_3))
  (Rendering|Material|SetScalarParameterValue "/Game/MaterialParameterCollections/MPC_Weather.MPC_Weather" "LightningIntensity" (Math|Float|Clamp(Float) (/ (- (Variables|WeatherTypes|GetWeatherIntensity) 0.75) 0.25)) :!class /Script/Engine.KismetMaterialLibrary)
  (switch Utilities|FlowControl|Switch|SwitchonE_WeatherType (Variables|WeatherTypes|GetCurrentWeather)
    (:NewEnumerator0
      (Rendering|Material|SetScalarParameterValue "/Game/MaterialParameterCollections/MPC_Weather.MPC_Weather" "FogDensity" 0.0 :!class /Script/Engine.KismetMaterialLibrary :!label _label))
    (:NewEnumerator1
      (goto _label))
    (:NewEnumerator2
      (goto _label))
    (:NewEnumerator3
      (goto _label))
    (:NewEnumerator4
      (goto _label))
    (:NewEnumerator5
      (Rendering|Material|SetScalarParameterValue "/Game/MaterialParameterCollections/MPC_Weather.MPC_Weather" "FogDensity" 0.7 :!class /Script/Engine.KismetMaterialLibrary)))
  (Rendering|Material|SetScalarParameterValue "/Game/MaterialParameterCollections/MPC_Ocean.MPC_Ocean" "GlobalWaveStrength" (Math|Float|Lerp 0.55 1.75 (Variables|WeatherTypes|GetWeatherIntensity)) :!class /Script/Engine.KismetMaterialLibrary)
  (Rendering|Material|SetScalarParameterValue "/Game/MaterialParameterCollections/MPC_Ocean.MPC_Ocean" "GlobalWaveSpeed" (Math|Float|Lerp 0.65 1.45 (Variables|WeatherTypes|GetWeatherIntensity)) :!class /Script/Engine.KismetMaterialLibrary)
  (Rendering|Material|SetScalarParameterValue "/Game/MaterialParameterCollections/MPC_Ocean.MPC_Ocean" "GlobalWaveSteepness" (Math|Float|Lerp 0.75 1.2 (Variables|WeatherTypes|GetWeatherIntensity)) :!class /Script/Engine.KismetMaterialLibrary)
  (Rendering|Material|SetScalarParameterValue "/Game/MaterialParameterCollections/MPC_Ocean.MPC_Ocean" "GlobalFoamStrength" (Math|Float|Lerp 0.5 1.6 (Variables|WeatherTypes|GetWeatherIntensity)) :!class /Script/Engine.KismetMaterialLibrary)
  (Rendering|Material|SetScalarParameterValue "/Game/MaterialParameterCollections/MPC_Ocean.MPC_Ocean" "WaterRoughness" (Math|Float|Lerp 0.12 0.6 (Variables|WeatherTypes|GetWeatherIntensity)) :!class /Script/Engine.KismetMaterialLibrary)
  (Rendering|Material|SetScalarParameterValue "/Game/MaterialParameterCollections/MPC_Ocean.MPC_Ocean" "WaterClarity" (Math|Float|Lerp 1.0 0.45 (Variables|WeatherTypes|GetWeatherIntensity)) :!class /Script/Engine.KismetMaterialLibrary)
  (Class|ExponentialHeightFogComponent|SetFogDensity _component (Variables|Fog|GetCurrentFogDensity))
  (Class|ExponentialHeightFogComponent|SetFogHeightFalloff _component (Variables|Fog|GetCurrentFogHeightFalloff))
  (Class|ExponentialHeightFogComponent|SetVolumetricFog _component true)
  (Rendering|Components|Light|SetIntensity (Variables|/Script/Engine.Light|GetLightComponent (Variables|Actors|GetSunLight)) (Variables|Light|GetCurrentSunIntensity))
  (Rendering|Components|Light|SetIntensity (Variables|/Script/Engine.SkyLight|GetLightComponent (Variables|Actors|GetSkyLight)) (Variables|Light|GetCurrentSkyLightIntensity))
  (Rendering|Material|SetScalarParameterValue "/Game/MaterialParameterCollections/MPC_Weather.MPC_Weather" "CloudCoverage" (Variables|Clouds|GetCurrentCloudCoverage) :!class /Script/Engine.KismetMaterialLibrary)
  (Rendering|Material|SetScalarParameterValue "/Game/MaterialParameterCollections/MPC_Weather.MPC_Weather" "StormCloudAmount" (Variables|Clouds|GetCurrentStormCloudAmount) :!class /Script/Engine.KismetMaterialLibrary))

(fn SetWeatherInstant
  (params (NewWeather :type E_WeatherType%20Enum :default "NewEnumerator0"))
  (Variables|Transition|SetIsTransitioning false)
  (Variables|Transition|SetTransitionProgress 1.0)
  (Variables|WeatherTypes|SetCurrentWeather NewWeather)
  (Variables|WeatherTypes|SetTargetWeather NewWeather)
  (bind _intensity (CallFunction|GetIntensityforWeather NewWeather))
  (Variables|WeatherTypes|SetWeatherIntensity _intensity)
  (Variables|Transition|SetStartingWeatherIntensity _intensity)
  (Variables|Transition|SetTargetWeatherIntensity _intensity)
  (CallFunction|SetTransitionValues)
  (CallFunction|SetCurrenttoTargetInstant)
  (CallFunction|ApplyWeatherValues)
  (Default|CallOnWeatherIntensityChanged (Variables|WeatherTypes|GetWeatherIntensity))
  (Default|CallOnWeatherChanged (Variables|WeatherTypes|GetCurrentWeather)))

(fn SetTransitionValues
  (Variables|Fog|SetStartFogDensity (Variables|Fog|GetCurrentFogDensity))
  (Variables|Fog|SetStartFogHeightFalloff (Variables|Fog|GetCurrentFogHeightFalloff))
  (Variables|Light|SetStartSunIntensity (Variables|Light|GetCurrentSunIntensity))
  (Variables|Light|SetStartSkyLightIntensity (Variables|Light|GetCurrentSkyLightIntensity))
  (Variables|Clouds|SetStartCloudCoverage (Variables|Clouds|GetCurrentCloudCoverage))
  (Variables|Rain|SetStartRainIntensity (Variables|Rain|GetCurrentRainIntensity))
  (switch Utilities|FlowControl|Switch|SwitchonE_WeatherType (Variables|WeatherTypes|GetTargetWeather)
    (:NewEnumerator0
      (Variables|Fog|SetTargetFogDensity 0.002)
      (Variables|Fog|SetTargetFogHeightFalloff 0.2)
      (Variables|Light|SetTargetSunIntensity 8.0)
      (Variables|Light|SetTargetSkyLightIntensity 1.0)
      (Variables|Clouds|SetTargetCloudCoverage -0.2)
      (Variables|Rain|SetTargetRainIntensity 0.0)
      (Variables|Clouds|SetTargetStormCloudAmount 0.0))
    (:NewEnumerator1
      (Variables|Fog|SetTargetFogDensity 0.008)
      (Variables|Fog|SetTargetFogHeightFalloff 0.18)
      (Variables|Light|SetTargetSunIntensity 4.0)
      (Variables|Light|SetTargetSkyLightIntensity 0.75)
      (Variables|Clouds|SetTargetCloudCoverage 0.65)
      (Variables|Rain|SetTargetRainIntensity 0.0)
      (Variables|Clouds|SetTargetStormCloudAmount 0.15))
    (:NewEnumerator2
      (Variables|Fog|SetTargetFogDensity 0.015)
      (Variables|Fog|SetTargetFogHeightFalloff 0.15)
      (Variables|Light|SetTargetSunIntensity 2.5)
      (Variables|Light|SetTargetSkyLightIntensity 0.55)
      (Variables|Clouds|SetTargetCloudCoverage 0.85)
      (Variables|Rain|SetTargetRainIntensity 0.55)
      (Variables|Clouds|SetTargetStormCloudAmount 0.4))
    (:NewEnumerator3
      (Variables|Fog|SetTargetFogDensity 0.025)
      (Variables|Fog|SetTargetFogHeightFalloff 0.12)
      (Variables|Light|SetTargetSunIntensity 1.2)
      (Variables|Light|SetTargetSkyLightIntensity 0.35)
      (Variables|Clouds|SetTargetCloudCoverage 1.0)
      (Variables|Rain|SetTargetRainIntensity 0.85)
      (Variables|Clouds|SetTargetStormCloudAmount 0.75))
    (:NewEnumerator4
      (Variables|Fog|SetTargetFogDensity 0.04)
      (Variables|Fog|SetTargetFogHeightFalloff 0.1)
      (Variables|Light|SetTargetSunIntensity 0.4)
      (Variables|Light|SetTargetSkyLightIntensity 0.2)
      (Variables|Clouds|SetTargetCloudCoverage 1.0)
      (Variables|Rain|SetTargetRainIntensity 1.0)
      (Variables|Clouds|SetTargetStormCloudAmount 1.0))
    (:NewEnumerator5
      (Variables|Fog|SetTargetFogDensity 0.1)
      (Variables|Fog|SetTargetFogHeightFalloff 0.08)
      (Variables|Light|SetTargetSunIntensity 1.5)
      (Variables|Light|SetTargetSkyLightIntensity 0.45)
      (Variables|Clouds|SetTargetCloudCoverage 0.5)
      (Variables|Rain|SetTargetRainIntensity 0.0)
      (Variables|Clouds|SetTargetStormCloudAmount 0.0))))

(fn SetCurrenttoTargetInstant
  (Variables|Fog|SetCurrentFogDensity (Variables|Fog|GetTargetFogDensity))
  (Variables|Fog|SetCurrentFogHeightFalloff (Variables|Fog|GetTargetFogHeightFalloff))
  (Variables|Light|SetCurrentSunIntensity (Variables|Light|GetTargetSunIntensity))
  (Variables|Light|SetCurrentSkyLightIntensity (Variables|Light|GetTargetSkyLightIntensity))
  (Variables|Clouds|SetCurrentCloudCoverage (Variables|Clouds|GetTargetCloudCoverage))
  (Variables|Rain|SetCurrentRainIntensity (Variables|Rain|GetTargetRainIntensity))
  (Variables|Clouds|SetCurrentStormCloudAmount (Variables|Clouds|GetTargetStormCloudAmount)))

(fn UpdateRainOceanParameters
  (bind _oceanmanager (Variables|Actors|GetOceanManager))
  (bind _ns_rain (Variables|Default|GetNS_Rain))
  (bind _ns_rain_2 (Variables|Default|GetNS_Rain))
  (bind _oceanmanager_2 (Variables|Actors|GetOceanManager))
  (bind _wavea (Variables|/Game/Blueprints/Managers/BP_OceanManager.BP_OceanManager_C|GetWaveA _oceanmanager))
  (bind _waveb (Variables|/Game/Blueprints/Managers/BP_OceanManager.BP_OceanManager_C|GetWaveB _oceanmanager_2))
  (Niagara|SetNiagaraVariable(Float) (Variables|Default|GetNS_Rain) "User.GlobalWaveStrength" (Variables|/Game/Blueprints/Managers/BP_OceanManager.BP_OceanManager_C|GetGlobalWaveStrength (Variables|Actors|GetOceanManager)))
  (Niagara|SetNiagaraVariable(Float) (Variables|Default|GetNS_Rain) "User.OceanBaseHeight" (Variables|/Game/Blueprints/Managers/BP_OceanManager.BP_OceanManager_C|GetOceanBaseHeight (Variables|Actors|GetOceanManager)))
  (Niagara|SetNiagaraVariable(Float) (Variables|Default|GetNS_Rain) "User.OceanTime" (Variables|/Game/Blueprints/Managers/BP_OceanManager.BP_OceanManager_C|GetOceanTime (Variables|Actors|GetOceanManager)))
  (Niagara|SetNiagaraVariable(Vector3) (Variables|Default|GetNS_Rain) "User.WaveADirection" (Math|Conversions|ToVector(Vector2D) (.direction _wavea)))
  (Niagara|SetNiagaraVariable(Float) (Variables|Default|GetNS_Rain) "User.WaveAAmplitude" (.amplitude _wavea))
  (Niagara|SetNiagaraVariable(Float) (Variables|Default|GetNS_Rain) "User.WaveAWavelength" (.wavelength _wavea))
  (Niagara|SetNiagaraVariable(Float) _ns_rain_2 "User.WaveASpeed" (.speed _wavea))
  (Niagara|SetNiagaraVariable(Float) _ns_rain_2 "User.WaveASteepness" (.steepness _wavea))
  (Niagara|SetNiagaraVariable(Vector3) (Variables|Default|GetNS_Rain) "User.WaveBDirection" (Math|Conversions|ToVector(Vector2D) (.direction _waveb)))
  (Niagara|SetNiagaraVariable(Float) (Variables|Default|GetNS_Rain) "User.WaveBAmplitude" (.amplitude _waveb))
  (Niagara|SetNiagaraVariable(Float) (Variables|Default|GetNS_Rain) "User.WaveBWavelength" (.wavelength _waveb))
  (Niagara|SetNiagaraVariable(Float) _ns_rain "User.WaveBSpeed" (.speed _waveb))
  (Niagara|SetNiagaraVariable(Float) _ns_rain "User.WaveBSteepness" (.steepness _waveb)))

(fn TriggerLightningStrike
  (bind _returnvalue (Game|Player|GetPlayerPawn 0))
  (bind _returnvalue_2 (Math|Random|RandomFloatinRange 4e+03 1.2e+04))
  (bind _returnvalue_3 (Math|Random|RandomFloatinRange 0.0 3.6e+02))
  (bind _returnvalue_4 (Math|Vector|MakeVector 0.0 0.0 1e+04))
  (bind _returnvalue_5 (Transformation|GetActorLocation _returnvalue))
  (bind _returnvalue_6 (Math|Rotator|MakeRotator 0.0 0.0 _returnvalue_3))
  (bind _returnvalue_7 (Math|Vector|GetForwardVector _returnvalue_6))
  (bind _returnvalue_8 (* _returnvalue_2 _returnvalue_7))
  (bind _returnvalue_9 (+ _returnvalue_5 _returnvalue_8))
  (bind (_x _y) (Math|Vector|BreakVector _returnvalue_9))
  (bind _outhit (Collision|LineTraceByChannel (+ _returnvalue_4 _returnvalue_9) (- _returnvalue_4 _returnvalue_9) "TraceTypeQuery1" false 0 "ForDuration"))
  (Niagara|SpawnSystematLocation "/Game/Niagara/NS_LightningStrike.NS_LightningStrike" (Math|Vector|SelectVector (.ImpactPoint (Collision|BreakHitResult _outhit)) (Math|Vector|MakeVector _x _y (Variables|/Game/Blueprints/Managers/BP_OceanManager.BP_OceanManager_C|GetOceanBaseHeight (Variables|Actors|GetOceanManager))) (.bBlockingHit (Collision|BreakHitResult _outhit))) (Math|Rotator|MakeRotator 0.0 0.0 (Math|Random|RandomFloatinRange 0.0 3.6e+02)))
  (return (Math|Vector|SelectVector (.ImpactPoint (Collision|BreakHitResult _outhit)) (Math|Vector|MakeVector _x _y (Variables|/Game/Blueprints/Managers/BP_OceanManager.BP_OceanManager_C|GetOceanBaseHeight (Variables|Actors|GetOceanManager))) (.bBlockingHit (Collision|BreakHitResult _outhit)))))
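; Debug actor that visualizes the ocean's wave surface as a grid of points around the player pawn.
; On BeginPlay it finds the BP_OceanManager, then redraws every Tick while ShowWaveGrid is enabled.
; DrawWaveGrid samples water height across a configurable square grid centered on the pawn's location, drawing a point at each wave height and a line to it from the ocean base height.
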(event EventBeginPlay
  (bind _returnvalue (Actor|GetActorOfClass "/Game/Blueprints/Managers/BP_OceanManager.BP_OceanManager_C"))
  (Variables|Default|SetOceanManager _returnvalue))

(event EventTick
  (params (DeltaSeconds :type Float%20%28single-precision%29))
  (if (Variables|Default|GetShowWaveGrid)
    (CallFunction|DrawWaveGrid)))

(fn ConstructionScript)

(fn DrawWaveGrid
  (bind _gridhalfsize (Variables|Default|GetGridHalfSize))
  (bind _gridhalfsize_2 (Variables|Default|GetGridHalfSize))
  (bind _returnvalue (* -1 _gridhalfsize_2))
  (Utilities|IsValid (Variables|Default|GetOceanManager)
    (:Is%20Valid
      (for _index (range _returnvalue _gridhalfsize)
        (for _index_2 (range _returnvalue _gridhalfsize)
          (bind _oceansample (Default|GetOceanSampleatLocation (Variables|Default|GetOceanManager) (+ (Math|Vector|MakeVector (* _index (Variables|Default|GetGridSpacing)) (* _index_2 (Variables|Default|GetGridSpacing)) 0.0) (Transformation|GetActorLocation (Game|Player|GetPlayerPawn 0)))))
          (bind _oceanheight (Default|GetOceanBaseHeight (Variables|Default|GetOceanManager)))
          (Rendering|Debug|DrawDebugPoint (Math|Vector|MakeVector (.X (Math|Vector|BreakVector (+ (Math|Vector|MakeVector (* _index (Variables|Default|GetGridSpacing)) (* _index_2 (Variables|Default|GetGridSpacing)) 0.0) (Transformation|GetActorLocation (Game|Player|GetPlayerPawn 0))))) (.Y (Math|Vector|BreakVector (+ (Math|Vector|MakeVector (* _index (Variables|Default|GetGridSpacing)) (* _index_2 (Variables|Default|GetGridSpacing)) 0.0) (Transformation|GetActorLocation (Game|Player|GetPlayerPawn 0))))) (.waterheight _oceansample)) (Variables|Default|GetDebugPointSize) "(R=0.160327,G=0.949354,B=1.000000,A=1.000000)" 0.0)
          (Rendering|Debug|DrawDebugLine (Math|Vector|MakeVector (.X (Math|Vector|BreakVector (+ (Math|Vector|MakeVector (* _index (Variables|Default|GetGridSpacing)) (* _index_2 (Variables|Default|GetGridSpacing)) 0.0) (Transformation|GetActorLocation (Game|Player|GetPlayerPawn 0))))) (.Y (Math|Vector|BreakVector (+ (Math|Vector|MakeVector (* _index (Variables|Default|GetGridSpacing)) (* _index_2 (Variables|Default|GetGridSpacing)) 0.0) (Transformation|GetActorLocation (Game|Player|GetPlayerPawn 0))))) _oceanheight) (Math|Vector|MakeVector (.X (Math|Vector|BreakVector (+ (Math|Vector|MakeVector (* _index (Variables|Default|GetGridSpacing)) (* _index_2 (Variables|Default|GetGridSpacing)) 0.0) (Transformation|GetActorLocation (Game|Player|GetPlayerPawn 0))))) (.Y (Math|Vector|BreakVector (+ (Math|Vector|MakeVector (* _index (Variables|Default|GetGridSpacing)) (* _index_2 (Variables|Default|GetGridSpacing)) 0.0) (Transformation|GetActorLocation (Game|Player|GetPlayerPawn 0))))) (.waterheight _oceansample)) "(R=0.000000,G=0.128739,B=1.000000,A=1.000000)" 0.0 2.0))))))
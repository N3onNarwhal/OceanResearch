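; Ocean manager that holds global ocean state and mirrors it into the MPC_Ocean Material Parameter Collection.
; BeginPlay pushes all wave, foam, current and water settings, while Tick advances a scaled, resettable OceanTime in the collection.
; Runtime setters update waves, current and clarity with clamping and fire OnOceanSettingsChanged.
; SetCurrent validates and clamps only its stored values, sending raw inputs to the collection.
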(event EventBeginPlay
  (CallFunction|ApplyOceanSettings))

(event EventTick
  (params (DeltaSeconds :type Float%20%28single-precision%29))
  (CallFunction|UpdateOceanTime DeltaSeconds))

(fn ConstructionScript)

(fn ApplyOceanSettings
  (bind _globalcurrentdirection (Variables|Default|GetGlobalCurrentDirection))
  (Rendering|Material|SetScalarParameterValue "/Game/MaterialParameterCollections/MPC_Ocean.MPC_Ocean" "OceanBaseHeight" (Variables|Default|GetOceanBaseHeight) :!class /Script/Engine.KismetMaterialLibrary)
  (Rendering|Material|SetScalarParameterValue "/Game/MaterialParameterCollections/MPC_Ocean.MPC_Ocean" "GlobalWaveStrength" (Variables|Default|GetGlobalWaveStrength) :!class /Script/Engine.KismetMaterialLibrary)
  (Rendering|Material|SetScalarParameterValue "/Game/MaterialParameterCollections/MPC_Ocean.MPC_Ocean" "GlobalWaveSpeed" (Variables|Default|GetGlobalWaveSpeed) :!class /Script/Engine.KismetMaterialLibrary)
  (Rendering|Material|SetScalarParameterValue "/Game/MaterialParameterCollections/MPC_Ocean.MPC_Ocean" "GlobalWaveSteepness" (Variables|Default|GetGlobalWaveSteepness) :!class /Script/Engine.KismetMaterialLibrary)
  (Rendering|Material|SetScalarParameterValue "/Game/MaterialParameterCollections/MPC_Ocean.MPC_Ocean" "GlobalFoamStrength" (Variables|Default|GetGlobalFoamStrength) :!class /Script/Engine.KismetMaterialLibrary)
  (Rendering|Material|SetScalarParameterValue "/Game/MaterialParameterCollections/MPC_Ocean.MPC_Ocean" "GlobalCurrentStrength" (Variables|Default|GetGlobalCurrentStrength) :!class /Script/Engine.KismetMaterialLibrary)
  (Rendering|Material|SetScalarParameterValue "/Game/MaterialParameterCollections/MPC_Ocean.MPC_Ocean" "WaterClarity" (Variables|Default|GetWaterClarity) :!class /Script/Engine.KismetMaterialLibrary)
  (Rendering|Material|SetScalarParameterValue "/Game/MaterialParameterCollections/MPC_Ocean.MPC_Ocean" "WaterRoughness" (Variables|Default|GetWaterRoughness) :!class /Script/Engine.KismetMaterialLibrary)
  (Rendering|Material|SetVectorParameterValue "/Game/MaterialParameterCollections/MPC_Ocean.MPC_Ocean" "GlobalCurrentDirection" (Utilities|Struct|MakeLinearColor (.x _globalcurrentdirection) (.y _globalcurrentdirection) (.z _globalcurrentdirection) 1.0) :!class /Script/Engine.KismetMaterialLibrary)
  (Default|CallOnOceanSettingsChanged))

(fn SetWaveStrength
  (params (NewStrength :type Float%20%28double-precision%29))
  (bind _output_get (Variables|Default|SetGlobalWaveStrength (Math|Float|Clamp(Float) NewStrength 0.0 3.0)))
  (Rendering|Material|SetScalarParameterValue "/Game/MaterialParameterCollections/MPC_Ocean.MPC_Ocean" "GlobalWaveStrength" _output_get :!class /Script/Engine.KismetMaterialLibrary)
  (Default|CallOnOceanSettingsChanged))

(fn SetWaveSpeed
  (params (NewSpeed :type Float%20%28double-precision%29))
  (bind _output_get (Variables|Default|SetGlobalWaveSpeed (Math|Float|Clamp(Float) NewSpeed 0.0 3.0)))
  (Rendering|Material|SetScalarParameterValue "/Game/MaterialParameterCollections/MPC_Ocean.MPC_Ocean" "GlobalWaveSpeed" _output_get :!class /Script/Engine.KismetMaterialLibrary)
  (Default|CallOnOceanSettingsChanged))

(fn SetCurrent
  (params (NewStrength :type Float%20%28double-precision%29) (NewDirection :type Vector))
  (if (> (Math|Vector|VectorLength NewDirection) 0.001)
    (Variables|Default|SetGlobalCurrentDirection NewDirection))
  (Variables|Default|SetGlobalCurrentStrength (Math|Float|Clamp(Float) NewStrength 0.0 2e+03))
  (Rendering|Material|SetVectorParameterValue "/Game/MaterialParameterCollections/MPC_Ocean.MPC_Ocean" "GlobalCurrentDirection" (Utilities|Struct|MakeLinearColor (.x NewDirection) (.y NewDirection) (.z NewDirection) 1.0) :!class /Script/Engine.KismetMaterialLibrary)
  (Rendering|Material|SetScalarParameterValue "/Game/MaterialParameterCollections/MPC_Ocean.MPC_Ocean" "GlobalCurrentStrength" NewStrength :!class /Script/Engine.KismetMaterialLibrary)
  (Default|CallOnOceanSettingsChanged))

(fn SetWaterClarity
  (params (NewClarity :type Float%20%28double-precision%29))
  (bind _output_get (Variables|Default|SetWaterClarity (Math|Float|Clamp(Float) NewClarity)))
  (Rendering|Material|SetScalarParameterValue "/Game/MaterialParameterCollections/MPC_Ocean.MPC_Ocean" "WaterClarity" _output_get :!class /Script/Engine.KismetMaterialLibrary)
  (Default|CallOnOceanSettingsChanged))

(fn GetOceanBaseHeight
  (return (Variables|Default|GetOceanBaseHeight)))

(fn ResetOceanTime
  (bind _output_get (Variables|Default|SetOceanTime 0.0))
  (Rendering|Material|SetScalarParameterValue "/Game/MaterialParameterCollections/MPC_Ocean.MPC_Ocean" "OceanTime" _output_get :!class /Script/Engine.KismetMaterialLibrary))

(fn UpdateOceanTime
  (params (DeltaSeconds :type Float%20%28double-precision%29))
  (bind _output_get (Variables|Default|SetOceanTime (+ (* DeltaSeconds (Variables|Default|GetOceanTimeScale)) (Variables|Default|GetOceanTime))))
  (Rendering|Material|SetScalarParameterValue "/Game/MaterialParameterCollections/MPC_Ocean.MPC_Ocean" "OceanTime" _output_get :!class /Script/Engine.KismetMaterialLibrary))
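; Weather manager that holds the current weather state and switches between clear, cloudy, rain, storm, heavy storm and fog.
; Each weather type maps to a single intensity value, written to the MPC_Weather material parameter collection.
; Changes are instant or blended by a timeline whose play rate is scaled to the requested duration.
; Event dispatchers announce transition start, intensity changes and completed weather changes.
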(event Custom|TransitionToWeather
  (params (NewWeather :type E_WeatherType%20Enum :default "NewEnumerator0") (Duration :type Float%20%28double-precision%29))
  (if (<= Duration 0.01)
    (CallFunction|SetWeatherInstant NewWeather)
    (else
      (Variables|Default|SetStartingWeatherIntensity (Variables|Default|GetWeatherIntensity))
      (Variables|Default|SetTargetWeather NewWeather)
      (Variables|Default|SetTransitionDuration Duration)
      (Variables|Default|SetTransitionProgress 0.0)
      (Variables|Default|SetIsTransitioning true)
      (bind _intensity (CallFunction|GetIntensityforWeather (Variables|Default|GetTargetWeather)))
      (Variables|Default|SetTargetWeatherIntensity _intensity)
      (Default|CallOnWeatherTransitionStarted (Variables|Default|GetCurrentWeather) (Variables|Default|GetTargetWeather) (Variables|Default|GetTransitionDuration))
      (Components|Timeline|SetPlayRate (Variables|Default|GetTI_WeatherTransition) (/ 1.0 (Variables|Default|GetTransitionDuration)))
      (bind _transitionalpha (Timeline|TI_WeatherTransition PlayFromStart)
        (:Update
          (Variables|Default|SetTransitionProgress _transitionalpha)
          (bind _output_get (Variables|Default|SetWeatherIntensity (Math|Float|Lerp (Variables|Default|GetStartingWeatherIntensity) (Variables|Default|GetTargetWeatherIntensity) (Variables|Default|GetTransitionProgress))))
          (CallFunction|ApplyWeatherValues)
          (Default|CallOnWeatherIntensityChanged _output_get))
        (:Finished
          (Variables|Default|SetWeatherIntensity (Variables|Default|GetTargetWeatherIntensity))
          (Variables|Default|SetCurrentWeather (Variables|Default|GetTargetWeather))
          (Variables|Default|SetTransitionProgress 1.0)
          (Variables|Default|SetIsTransitioning false)
          (CallFunction|ApplyWeatherValues)
          (Default|CallOnWeatherChanged (Variables|Default|GetCurrentWeather)))))))

(event EventBeginPlay
  (CallFunction|SetWeatherInstant (Variables|Default|GetStartingWeather)))

(fn ConstructionScript)

(fn GetIntensityforWeather
  (params (Weather :type E_WeatherType%20Enum :default "NewEnumerator0"))
  (switch Utilities|FlowControl|Switch|SwitchonE_WeatherType Weather
    (:NewEnumerator0
      (return 0.0))
    (:NewEnumerator1
      (return 0.25))
    (:NewEnumerator2
      (return 0.5))
    (:NewEnumerator3
      (return 0.8))
    (:NewEnumerator4
      (return 1.0))
    (:NewEnumerator5
      (return 0.35))))

(fn ApplyWeatherValues
  (Rendering|Material|SetScalarParameterValue "/Game/MaterialParameterCollections/MPC_Weather.MPC_Weather" "WeatherIntensity" (Variables|Default|GetWeatherIntensity) :!class /Script/Engine.KismetMaterialLibrary))

(fn SetWeatherInstant
  (params (NewWeather :type E_WeatherType%20Enum :default "NewEnumerator0"))
  (Variables|Default|SetIsTransitioning false)
  (Variables|Default|SetTransitionProgress 1.0)
  (Variables|Default|SetCurrentWeather NewWeather)
  (Variables|Default|SetTargetWeather NewWeather)
  (bind _intensity (CallFunction|GetIntensityforWeather NewWeather))
  (Variables|Default|SetWeatherIntensity _intensity)
  (CallFunction|ApplyWeatherValues)
  (Default|CallOnWeatherIntensityChanged (Variables|Default|GetWeatherIntensity))
  (Default|CallOnWeatherChanged (Variables|Default|GetCurrentWeather)))
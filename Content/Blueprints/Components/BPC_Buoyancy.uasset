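; BPC_Buoyancy is a component that floats its owner's physics static mesh on the surface reported by BP_OceanManager.
; Each tick it samples the ocean at scene components tagged BuoyancyPoint.
; Submerged points receive vertical spring forces from depth plus a height offset, damped by point velocity, with strength and damping split across all points.
; Horizontal drag pulls the body toward the last sampled water velocity, even when no point is submerged.
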(event EventBeginPlay
  (Variables|Default|SetAffectedPrimitive (Actor|GetComponentbyClass (Components|GetOwner) "/Script/Engine.StaticMeshComponent"))
  (bind _returnvalue (Actor|GetActorOfClass "/Game/Blueprints/Managers/BP_OceanManager.BP_OceanManager_C"))
  (Variables|Default|SetOceanManager _returnvalue)
  (Variables|Default|SetBuoyancyPoints (Actor|GetComponentsbyTag (Components|GetOwner) "/Script/Engine.SceneComponent" "BuoyancyPoint")))

(event EventTick
  (params (DeltaSeconds :type Float%20%28single-precision%29))
  (if (and (Utilities|IsValid (Variables|Default|GetAffectedPrimitive)) (Utilities|IsValid (Variables|Default|GetOceanManager)))
    (CallFunction|ApplyBuoyancy DeltaSeconds)))

(fn ApplyBuoyancy
  (params (DeltaSeconds :type Float%20%28double-precision%29))
  (for _array_element (Variables|Default|GetBuoyancyPoints)
    (bind _output_get (LocalVariables|SetSamplePoint (Transformation|GetWorldLocation _array_element)))
    (bind _oceansample (Default|GetOceanSampleatLocation (Variables|Default|GetOceanManager) _output_get))
    (LocalVariables|SetWaterVelocity (.horizontalvelocity _oceansample))
    (bind _output_get_2 (LocalVariables|SetTargetSurfaceHeight (+ (.waterheight _oceansample) (Variables|Default|GetFloatHeightOffset))))
    (bind _output_get_3 (LocalVariables|SetSubmersionDepth (- _output_get_2 (.z (LocalVariables|GetSamplePoint)))))
    (if (> _output_get_3 0.0)
      (bind _returnvalue (Class|PrimitiveComponent|GetPhysicsLinearVelocityatPoint (Variables|Default|GetAffectedPrimitive) (LocalVariables|GetSamplePoint) "None"))
      (LocalVariables|SetVerticalDamping (* (.Z (Math|Vector|BreakVector _returnvalue)) (Variables|Default|GetBuoyancyDamping)))
      (Class|PrimitiveComponent|AddForceatLocation (Variables|Default|GetAffectedPrimitive) (Math|Vector|MakeVector 0.0 0.0 (- (* (LocalVariables|GetSubmersionDepth) (/ (Variables|Default|GetBuoyancyStrength) (Utilities|Array|Length (Variables|Default|GetBuoyancyPoints)))) (/ (LocalVariables|GetVerticalDamping) (Utilities|Array|Length (Variables|Default|GetBuoyancyPoints))))) (LocalVariables|GetSamplePoint) "None")))
  ;[0.15 0.15 0.15 0.5] Horizontal drag
  (bind _returnvalue_2 (Physics|GetPhysicsLinearVelocity (Variables|Default|GetAffectedPrimitive) "None"))
  (LocalVariables|SetObjectVelocity (Math|Vector|MakeVector (.x _returnvalue_2) (.y _returnvalue_2) 0.0))
  (LocalVariables|SetWaterVelocity (Math|Vector|MakeVector (.x (LocalVariables|GetWaterVelocity)) (.y (LocalVariables|GetWaterVelocity)) 0.0))
  (bind _output_get_4 (LocalVariables|SetRelativeVelocity (- (LocalVariables|GetObjectVelocity) (LocalVariables|GetWaterVelocity))))
  (Physics|AddForce (Variables|Default|GetAffectedPrimitive) (* _output_get_4 (Variables|Default|GetWaterDrag) -1.0) "None" true))
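; BP_GameState is a game state Blueprint that gives access to the world's ocean and weather managers and tracks a research score.
; The manager getters lazily find BP_OceanManager and BP_WeatherManager with GetActorOfClass when the cached reference is invalid, then return it.
; AddResearchScore adds a given amount to the running research score, and the event graph holds no active logic.
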(event EventBeginPlay)

(event EventTick
  (params (DeltaSeconds :type Float%20%28single-precision%29)))

(fn ConstructionScript)

(fn RegisterOceanManager
  (bind _returnvalue (Actor|GetActorOfClass "/Game/Blueprints/Managers/BP_OceanManager.BP_OceanManager_C"))
  (Variables|Default|SetOceanManager _returnvalue))

(fn RegisterWeatherManager
  (bind _returnvalue (Actor|GetActorOfClass "/Game/Blueprints/Managers/BP_WeatherManager.BP_WeatherManager_C"))
  (Variables|Default|SetWeatherManager _returnvalue))

(fn AddResearchScore
  (params (AddScore :type Integer))
  (Variables|Default|SetCurrentResearchScore (+ AddScore (Variables|Default|GetCurrentResearchScore))))

(fn GetOceanManager
  (bind _oceanmanager (Variables|Default|GetOceanManager))
  (Utilities|IsValid _oceanmanager
    (:Is%20Valid
      _)
    (:Is%20Not%20Valid
      (CallFunction|RegisterOceanManager)))
  (return _oceanmanager))

(fn GetWeatherManager
  (bind _weathermanager (Variables|Default|GetWeatherManager))
  (Utilities|IsValid _weathermanager
    (:Is%20Valid
      _)
    (:Is%20Not%20Valid
      (CallFunction|RegisterWeatherManager)))
  (return _weathermanager))
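; BP_Boat is a player-possessed, physics-driven boat that adds the IMC_Boat input mapping on possession.
; Each tick, throttle input applies engine force at the propeller point, cut off beyond separate forward and reverse speed limits.
; Steering applies mass-independent yaw torque, scaled by forward speed and inverted when moving backwards.
; A counter-torque proportional to yaw angular velocity damps turning every tick.
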(event Input|EnhancedActionEvents|EnhancedInputActionIA_Throttle
  (params (ActionValue :type Float%20%28double-precision%29) (ElapsedSeconds :type Float%20%28double-precision%29) (TriggeredSeconds :type Float%20%28double-precision%29) (InputAction :type Input%20Action%20Object%20Reference :default "/Game/Blueprints/Boat/IA_Throttle.IA_Throttle"))
  (:Triggered
    (Variables|Default|SetThrottleInput ActionValue))
  (:Completed
    (Variables|Default|SetThrottleInput 0.0)))

(event Input|EnhancedActionEvents|EnhancedInputActionIA_Steer
  (params (ActionValue :type Float%20%28double-precision%29) (ElapsedSeconds :type Float%20%28double-precision%29) (TriggeredSeconds :type Float%20%28double-precision%29) (InputAction :type Input%20Action%20Object%20Reference :default "/Game/Blueprints/Boat/IA_Steer.IA_Steer"))
  (:Triggered
    (Variables|Default|SetSteerInput ActionValue))
  (:Completed
    (Variables|Default|SetSteerInput 0.0)))

(event EventTick
  (params (DeltaSeconds :type Float%20%28single-precision%29))
  (CallFunction|ApplyThrottle)
  (CallFunction|ApplySteering)
  (CallFunction|ApplyYawDrag))

(event EventPossessed
  (params (NewController :type Controller%20Object%20Reference))
  (bind _asplayer_controller (Utilities|Casting|CastToPlayerController NewController))
  (Input|AddMappingContext (PlayerController|LocalPlayerSubsystems|GetEnhancedInputLocalPlayerSubsystem _asplayer_controller) "/Game/Blueprints/Boat/IMC_Boat.IMC_Boat" 0 "(bIgnoreAllPressedKeysUntilRelease=True,bForceImmediately=False,bNotifyUserSettings=False)"))

(fn ConstructionScript)

(fn GetForwardSpeed
  (bind _returnvalue (Physics|GetPhysicsLinearVelocity (Variables|Default|GetSM_Boat) "None"))
  (return (Math|Vector|DotProduct _returnvalue (Math|Vector|GetForwardVector (Variables|Default|GetMovementDirection)))))

(fn ApplyThrottle
  (if (> (Math|Float|Absolute(Float) (Variables|Default|GetThrottleInput)) 0.01)
    (bind _forwardspeed (CallFunction|GetForwardSpeed))
    (if (> (Variables|Default|GetThrottleInput) 0.0)
      (if (< _forwardspeed (Variables|Default|GetMaxForwardSpeed))
        (Class|PrimitiveComponent|AddForceatLocation (Variables|Default|GetSM_Boat) (* (Math|Vector|GetForwardVector (Variables|Default|GetMovementDirection)) (Variables|Default|GetThrottleInput) (Variables|Default|GetEngineForce)) (Transformation|GetWorldLocation (Variables|Default|GetPropellerPoint)) "None" :!label _label))
      (elif (< (Variables|Default|GetThrottleInput) 0.0)
        (if (> _forwardspeed (* (Variables|Default|GetMaxReverseSpeed) -1.0))
          (goto _label))))))

(fn GetSteeringEffectiveness
  (bind _forwardspeed (CallFunction|GetForwardSpeed))
  (return (Math|Float|MapRangeClamped (Math|Float|Absolute(Float) _forwardspeed) (Variables|Default|GetMinSteeringSpeed) (Variables|Default|GetFullSteeringSpeed) 0.0 1.0)))

(fn ApplySteering
  (bind _sm_boat (Variables|Default|GetSM_Boat))
  (if (> (Math|Float|Absolute(Float) (Variables|Default|GetSteerInput)) 0.01)
    (bind _forwardspeed (CallFunction|GetForwardSpeed))
    (bind _steeringeffectiveness (CallFunction|GetSteeringEffectiveness))
    (Class|PrimitiveComponent|AddTorqueinRadians _sm_boat (* (Math|Vector|GetUpVector _sm_boat) (* (Math|Float|SelectFloat -1.0 1.0 (< _forwardspeed 0.0)) (Variables|Default|GetSteerInput) (Variables|Default|GetSteeringTorque) _steeringeffectiveness)) "None" true)))

(fn ApplyYawDrag
  (bind _sm_boat (Variables|Default|GetSM_Boat))
  (Class|PrimitiveComponent|AddTorqueinRadians (Variables|Default|GetSM_Boat) (* (Math|Vector|GetUpVector (Variables|Default|GetSM_Boat)) (* (Math|Vector|DotProduct (Class|PrimitiveComponent|GetPhysicsAngularVelocityinRadians _sm_boat "None") (Math|Vector|GetUpVector _sm_boat)) (Variables|Default|GetYawDragStrength) -1.0)) "None" true))